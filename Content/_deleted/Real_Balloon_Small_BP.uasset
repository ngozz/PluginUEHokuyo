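; A small balloon actor that drifts upward, gets a random color and can be destroyed by a hit.
; On BeginPlay it disables mesh shadows, sets a randomized rising, sideways physics velocity and randomizes the BalloonColor material parameter within limited ranges.
; It destroys itself after a fixed delay, or earlier through GotHit, which spawns an emitter before destruction and has no caller in this Blueprint.
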(event EventBeginPlay
  (Rendering|SetCastShadow (Variables|Default|GetBalloonMesh) false)
  (Physics|SetPhysicsLinearVelocity (Variables|Default|GetBalloonMesh) (Math|Vector|MakeVector (Math|Random|RandomFloatinRange 0.0 0.0) (Math|Random|RandomFloatinRange 13.0 15.0) (Math|Random|RandomFloatinRange 25.0 5e+01)) false "None")
  (Rendering|Material|SetVectorParameterValueonMaterials (Variables|Default|GetBalloonMesh) "BalloonColor" (Math|Vector|MakeVector (Math|Random|RandomFloatinRange 0.0 0.12) (Math|Random|RandomFloatinRange 0.0 1.0) (Math|Random|RandomFloatinRange 0.5 1.0)))
  (Utilities|FlowControl|Delay 3e+01)
  (Actor|DestroyActor))

(event Collision|EventActorBeginOverlap
  (params (OtherActor :type Actor%20Object%20Reference)))

(event EventTick
  (params (DeltaSeconds :type Float%20%28single-precision%29)))

(fn ConstructionScript)

(fn GotHit
  (Effects|SpawnEmitteratLocation 0 "0, 0, 0")
  (Actor|DestroyActor))